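; Grenade projectile Blueprint that explodes on the first hit its sphere component registers, then destroys itself.
; The explosion spawns a particle emitter, applies radial damage and plays a sound, all at the actor's location.
; Damage radius comes from a variable, and damage is credited to the instigator's controller with the grenade as causer.
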(event OnComponentHit(Sphere)
  (params (HitComponent :type Primitive%20Component%20Object%20Reference) (OtherActor :type Actor%20Object%20Reference) (OtherComp :type Primitive%20Component%20Object%20Reference) (NormalImpulse :type Vector :default "0, 0, 0") (Hit :type Hit%20Result%20Structure%20%28by%20ref%29))
  (CallFunction|Explode)
  (Actor|DestroyActor))

(fn ConstructionScript)

(fn Explode
  (Effects|SpawnEmitteratLocation "/Game/WeaponEffects/Explosion/P_Explosion.P_Explosion" (Transformation|GetActorLocation))
  (Game|Damage|ApplyRadialDamage 1e+02 (Transformation|GetActorLocation) (Variables|Default|GetDamage%20Radius) 0 0 self (Game|GetInstigatorController) false "ECC_Visibility")
  (Audio|PlaySoundatLocation "/Game/Core/Sounds/Explosion_Cue.Explosion_Cue" (Transformation|GetActorLocation) "0, 0, 0" 1.0 1.0 0.0 0 0 0))