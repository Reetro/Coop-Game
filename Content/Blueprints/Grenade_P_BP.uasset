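; Grenade projectile actor that detonates on a one-second fuse after spawning, then destroys itself.
; BeginPlay waits out the delay and calls Explode, which spawns an explosion particle effect and sound at its location.
; Explode also applies radial damage within DamageRadius, credited to the instigator's controller, and draws a debug sphere showing the blast area.
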(event EventBeginPlay
  (Utilities|FlowControl|Delay 1.0)
  (CallFunction|Explode)
  (Actor|DestroyActor))

(fn ConstructionScript)

(fn Explode
  (Effects|SpawnEmitteratLocation "/Game/WeaponEffects/Explosion/P_Explosion.P_Explosion" (Transformation|GetActorLocation))
  (Game|Damage|ApplyRadialDamage 1e+02 (Transformation|GetActorLocation) (Variables|Default|GetDamage%20Radius) 0 0 self (Game|GetInstigatorController) false "ECC_Visibility")
  (Rendering|Debug|DrawDebugSphere (Transformation|GetActorLocation) (Variables|Default|GetDamage%20Radius) 12 "(R=1.000000,G=1.000000,B=1.000000,A=1.000000)" 1.0 5.0)
  (Audio|PlaySoundatLocation "/Game/Core/Explosion_Cue.Explosion_Cue" (Transformation|GetActorLocation) "0, 0, 0" 1.0 1.0 0.0 0 0 0))