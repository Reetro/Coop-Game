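; Behavior tree service that picks the AI pawn's combat target each tick.
; It scans actors known to the pawn's sight perception, skips friendlies and those with no health left in their SHealthComponent, and keeps the nearest.
; The chosen actor, or None if nothing qualifies, is written to a configurable Blackboard key.
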(event EventReceiveTickAI
  (params (OwnerController :type AI%20Controller%20Object%20Reference) (ControlledPawn :type Pawn%20Object%20Reference) (DeltaSeconds :type Float%20%28single-precision%29))
  (Variables|Default|SetBest%20Target%20Actor 0)
  (Variables|Default|SetNearest%20Target%20Distance 1e+06)
  (for _array_element (Class|AIPerceptionComponent|GetKnownPerceivedActors (Actor|GetComponentbyClass ControlledPawn "/Script/AIModule.AIPerceptionComponent") "/Script/AIModule.AISense_Sight")
    (Variables|Default|SetCurrent%20Array%20Element _array_element)
    (if (and (not (Class|SHealthComponent|IsFriendly _array_element ControlledPawn)) (> (Variables|/Script/CoopGame.SHealthComponent|GetHealth (Actor|GetComponentbyClass _array_element "/Script/CoopGame.SHealthComponent")) 0.0))
      (if (< (Math|Vector|VectorLength (- (Transformation|GetActorLocation ControlledPawn) (Transformation|GetActorLocation _array_element))) (Variables|Default|GetNearest%20Target%20Distance))
        (Variables|Default|SetNearest%20Target%20Distance (Math|Vector|VectorLength (- (Transformation|GetActorLocation ControlledPawn) (Transformation|GetActorLocation _array_element))))
        (Variables|Default|SetBest%20Target%20Actor (Variables|Default|GetCurrent%20Array%20Element)))))
  (Class|BTFunctionLibrary|SetBlackboardValueasObject (Variables|Default|GetBlackBoardKey) (Variables|Default|GetBest%20Target%20Actor)))