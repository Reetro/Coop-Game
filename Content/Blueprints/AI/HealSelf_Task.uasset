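; Behavior tree task that lets an AI-controlled pawn heal itself through its SHealthComponent.
; It applies HealPerTick, waits HealTickInterval, applies HealPerTick a second time, then finishes with success.
; When the pawn has no valid health component, it calls FinishAbort instead of finishing with failure.
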(event EventReceiveExecuteAI
  (params (OwnerController :type AI%20Controller%20Object%20Reference) (ControlledPawn :type Pawn%20Object%20Reference))
  (bind _returnvalue (Actor|GetComponentbyClass ControlledPawn "/Script/CoopGame.SHealthComponent"))
  (Utilities|IsValid _returnvalue
    (:Is%20Valid
      (bind _output_get (Variables|Default|SetHP%20Comp _returnvalue))
      (Class|SHealthComponent|Heal _output_get (Variables|Default|GetHeal%20Per%20Tick))
      (Utilities|FlowControl|Delay (Variables|Default|GetHeal%20Tick%20Interval))
      (Class|SHealthComponent|Heal (Variables|Default|GetHP%20Comp) (Variables|Default|GetHeal%20Per%20Tick))
      (AI|BehaviorTree|FinishExecute true))
    (:Is%20Not%20Valid
      (Class|BTTaskBlueprintBase|FinishAbort))))