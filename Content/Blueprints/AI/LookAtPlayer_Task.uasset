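; Behavior Tree task that snaps the controlled AI pawn to face a target actor, presumably the player, read from a Blackboard key.
; It sets the pawn's full rotation instantly to the look-at rotation from pawn location to target location, then finishes successfully.
; It aborts if the pawn or the target actor is invalid.
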(event EventReceiveExecuteAI
  (params (OwnerController :type AI%20Controller%20Object%20Reference) (ControlledPawn :type Pawn%20Object%20Reference))
  (bind _blackboardkey (Variables|Default|GetBlackBoardKey))
  (bind _returnvalue (AI|BehaviorTree|GetBlackboardValueasActor _blackboardkey))
  (bind _output_get (Variables|Default|SetCurrent%20Pawn ControlledPawn))
  (Utilities|IsValid _output_get
    (:Is%20Valid
      (Utilities|IsValid _returnvalue
        (:Is%20Valid
          (Transformation|SetActorRotation (Variables|Default|GetCurrent%20Pawn) (Math|Rotator|FindLookatRotation (Transformation|GetActorLocation (Variables|Default|GetCurrent%20Pawn)) (Transformation|GetActorLocation _returnvalue)))
          (AI|BehaviorTree|FinishExecute true))
        (:Is%20Not%20Valid
          (Class|BTTaskBlueprintBase|FinishAbort))))
    (:Is%20Not%20Valid
      (Class|BTTaskBlueprintBase|FinishAbort))))