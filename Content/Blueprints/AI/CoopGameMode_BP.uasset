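; Co-op game mode Blueprint that spawns enemy bots and tracks player score.
; SpawnNewBot runs an EQS spawn-location query and spawns a randomly chosen AdvancedAI or TrackerBot at each result, with debug spheres.
; An OnActorKilled binding stops weapon fire on non-player SCharacter victims and awards points to the killer's SPlayerState for non-player pawn kills, printing the score.
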(event Custom|OnQueryFinishedEvent
  (params (QueryInstance :type Env%20Query%20Instance%20Blueprint%20Wrapper%20Object%20Reference) (QueryStatus :type EEnvQueryStatus%20Enum :default "Processing"))
  ;[1 1 1] Spawn Enemies in waves
  (switch Utilities|FlowControl|Switch|SwitchonEEnvQueryStatus QueryStatus
    (:Success
      (bind _resultlocations (AI|EQS|GetQueryResultsasLocations QueryInstance))
      (for _array_element _resultlocations
        (Rendering|Debug|DrawDebugSphere _array_element 1e+02 12 "(R=1.000000,G=0.000000,B=0.026586,A=1.000000)" 2.0 2.0)
        (Game|SpawnActorfromClass (select (<= (Math|Random|RandomFloatinRange 0.0 1e+02) 35.0) "/Game/Blueprints/AI/AdvancedAI_BP.AdvancedAI_BP_C" "/Game/Blueprints/AI/TrackerBot_BP.TrackerBot_BP_C") (Math|Transform|MakeTransform _array_element) "AdjustIfPossibleButDontSpawnIfColliding" 0 0)))))

(event Custom|OnActorKilled_Event
  (params (VictimActor :type Actor%20Object%20Reference) (KillerActor :type Actor%20Object%20Reference) (KillerController :type Controller%20Object%20Reference))
  (bind _returnvalue (Pawn|GetControlledPawn KillerController))
  (bind _playerstate (Variables|/Script/Engine.Pawn|GetPlayerState _returnvalue))
  ;[1 1 1] Keep Track player score
  (Utilities|IsValid KillerController
    (:Is%20Valid
      (bind _aspawn (Utilities|Casting|CastToPawn VictimActor))
      (if (not (Pawn|IsPlayerControlled _aspawn))
        (bind _asscharacter (Utilities|Casting|CastToSCharacter _aspawn)
          (:then
            (Class|SWeapon|StopFire (Variables|/Script/CoopGame.SCharacter|GetCurrentWeapon _asscharacter)))
          (:CastFailed
            _))
        (Utilities|IsValid _returnvalue
          (:Is%20Valid
            (bind _assplayer_state (Utilities|Casting|CastToSPlayerState _playerstate)
              (:then
                (Class|SPlayerState|AddScore _assplayer_state 2e+01)
                (Development|PrintString (Utilities|String|ToString(Float) (Variables|/Script/Engine.PlayerState|GetScore _playerstate)) true true "(R=0.000000,G=1.000000,B=0.017634,A=1.000000)"))
              (:CastFailed
                (Development|PrintString "Unable to get player state in gamemode" true true "(R=1.000000,G=0.000000,B=0.010881,A=1.000000)")))))))))

(event EventBeginPlay
  ;[1 1 1] Keep Track player score
  (EventDispatchers|AssignOnActorKilled (delegate Custom|OnActorKilled_Event)))

(event EventSpawnNewBot
  ;[1 1 1] Spawn Enemies in waves
  (bind _returnvalue (AI|EQS|RunEQSQuery "/Game/Blueprints/AI/EQS_FIndSpawnLocation.EQS_FIndSpawnLocation" self "RandomBest25Pct"))
  (EventDispatchers|AssignOnQueryFinishedEvent _returnvalue (delegate Custom|OnQueryFinishedEvent)))

(fn ConstructionScript)