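; Ammo respawner actor that refills the ammo pickups inside its box volume once all of them are gone.
; On BeginPlay it saves the transforms of the overlapping SAmmoPickup actors and starts a fast looping timer.
; When the timer finds the box empty of pickups, it waits for RespawnDelay, then spawns an AmmoPickUp_BP at every saved transform.
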(event Custom|Respawn%20Ammo
  (if (<= (Utilities|Array|Length (Collision|GetOverlappingActors (Variables|Default|GetBox) "/Script/CoopGame.SAmmoPickup" :!class /Script/Engine.PrimitiveComponent)) 0)
    (Utilities|FlowControl|Delay (Variables|AmmoSpawning|GetRespawn%20Delay))
    (for _array_element (Variables|Default|GetSaved%20Transforms)
      (Game|SpawnActorfromClass "/Game/Blueprints/GameplayItems/AmmoPickUp_BP.AmmoPickUp_BP_C" _array_element "Undefined" 0 0))))

(event EventBeginPlay
  (for _array_element (Collision|GetOverlappingActors (Variables|Default|GetBox) "/Script/CoopGame.SAmmoPickup" :!class /Script/Engine.PrimitiveComponent)
    (Utilities|Array|Add (Variables|Default|GetSaved%20Transforms) (Transformation|GetActorTransform _array_element)))
  (Utilities|Time|SetTimerbyEvent (delegate Custom|Respawn%20Ammo) 0.01 true))

(fn ConstructionScript)